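; Interactable button that removes a Barrier actor when the player presses F while near it.
; Box overlap begin and end enable or disable player input and toggle the PressFToActivate prompt, without filtering the overlapping actor.
; F destroys the first Barrier found in the level, starts a timer with no function name, then destroys the button.
; Tick rotates the prompt along the camera-to-prompt direction with a small offset.
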(event `Key|F`
  (params (Key :type "Key Structure"))
  (:`Pressed`
    (bind _outactors (`GameplayStatics.GetAllActorsOfClass` "/Game/Blueprints/Barrier.Barrier_C"))
    (`self.K2_DestroyActor` (`|GetArrayItem` _outactors))
    (`KismetSystemLibrary.K2_SetTimer` null "" 0.5)
    (`self.K2_DestroyActor`)))

(event `self.Box.OnComponentBeginOverlap`
  (params (OverlappedComponent :type "PrimitiveComponent Object Reference") (OtherActor :type "Actor Object Reference") (OtherComp :type "PrimitiveComponent Object Reference") (OtherBodyIndex :type Integer) (bFromSweep :type Boolean) (SweepResult :type "HitResult Structure (by ref)"))
  (`self.EnableInput` (`GameplayStatics.GetPlayerController` 0))
  (`SceneComponent.ToggleVisibility` (`self.Press F to activate`) false :!label _label))

(event `self.Box.OnComponentEndOverlap`
  (params (OverlappedComponent :type "PrimitiveComponent Object Reference") (OtherActor :type "Actor Object Reference") (OtherComp :type "PrimitiveComponent Object Reference") (OtherBodyIndex :type Integer))
  (`self.DisableInput` (`GameplayStatics.GetPlayerController` 0))
  (goto _label))

(event `self.ReceiveTick`
  (params (DeltaSeconds :type "Float (single-precision)"))
  (bind _press_f_to_activate (`self.Press F to activate`))
  (`SceneComponent.K2_SetRelativeRotation` _press_f_to_activate (`KismetMathLibrary.ComposeRotators` (`KismetMathLibrary.MakeRotFromX` (- (`SceneComponent.K2_GetComponentLocation` _press_f_to_activate) (`self.K2_GetActorLocation` (`GameplayStatics.GetPlayerCameraManager` 0)))) (struct :`Yaw` 10.0)) false false))

(fn `UserConstructionScript`)
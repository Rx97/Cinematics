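; HorizontalMovingPlatform is a platform that moves a flattened cube along a spline path.
; On BeginPlay, a timeline plays and its Animation track, multiplied by the spline length, gives the distance at which the world location is sampled.
; Each update sets the cube's transform without sweep, keeping its current rotation and a fixed slab scale, so it does not turn to follow the spline.
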(event `self.ReceiveBeginPlay`
  (bind _spline (`self.Spline`))
  (bind (_direction _animation) (`Timeline|Timeline_0`)
    (:`Update`
      (`SceneComponent.K2_SetWorldTransform` (`self.Cube`) (`KismetMathLibrary.MakeTransform` (`SplineComponent.GetLocationAtDistanceAlongSpline` _spline (* _animation (`SplineComponent.GetSplineLength` _spline)) "World") (`SceneComponent.K2_GetComponentRotation` (`self.Cube`)) (2.125 2.125 0.125)) false false))))

(fn `UserConstructionScript`)
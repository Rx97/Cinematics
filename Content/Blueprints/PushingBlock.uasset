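; A pushing block obstacle that moves along a spline and launches the player.
; On BeginPlay, a timeline moves the cube along the spline by scaling its animation value by the spline length, keeping its rotation and setting a fixed scale.
; Any overlap with the box launches player character 0 by a LaunchVelocity variable, without checking which actor overlapped.
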(event `self.ReceiveBeginPlay`
  (bind _spline (`self.Spline`))
  (bind (_direction _animation) (`Timeline|Timeline_0`)
    (:`Update`
      (`SceneComponent.K2_SetWorldTransform` (`self.Cube`) (`KismetMathLibrary.MakeTransform` (`SplineComponent.GetLocationAtDistanceAlongSpline` _spline (* _animation (`SplineComponent.GetSplineLength` _spline)) "World") (`SceneComponent.K2_GetComponentRotation` (`self.Cube`)) (9.03125 3.15625 3.15625)) false false))))

(event `self.Box.OnComponentBeginOverlap`
  (params (OverlappedComponent :type "PrimitiveComponent Object Reference") (OtherActor :type "Actor Object Reference") (OtherComp :type "PrimitiveComponent Object Reference") (OtherBodyIndex :type Integer) (bFromSweep :type Boolean) (SweepResult :type "HitResult Structure (by ref)"))
  (if true
    (`Character.LaunchCharacter` (`GameplayStatics.GetPlayerCharacter` 0) (`self.LaunchVelocity`) false false)))

(fn `UserConstructionScript`)
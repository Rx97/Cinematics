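; An end-of-game trigger actor that plays a closing sequence and returns to the main menu.
; The first actor overlap, unfiltered by actor type, disables player input, plays MySequence and binds the re-enable event to its finish.
; Despite its name, that event leaves input disabled, starts MySequence2 and opens the mainMenu level immediately, without waiting for the second sequence to finish.
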(event `self.ReceiveActorBeginOverlap`
  (params (OtherActor :type "Actor Object Reference"))
  (bind _sequenceplayer (`LevelSequenceActor.SequencePlayer` (`self.mySequence`)))
  (`/Engine/EditorBlueprintResources/StandardMacros.DoOnce` false
    (:`Completed`
      (`self.DisableInput` (`GameplayStatics.GetPlayerCharacter` 0) (`GameplayStatics.GetPlayerController` 0))
      (`MovieSceneSequencePlayer.Play` _sequenceplayer)
      (add `MovieSceneSequencePlayer.OnFinished` _sequenceplayer (delegate `Re-enable`)))))

(event `Re-enable`
  (`MovieSceneSequencePlayer.Play` (`LevelSequenceActor.SequencePlayer` (`self.mySequence2`)))
  (`GameplayStatics.OpenLevel` "mainMenu"))

(fn `UserConstructionScript`)
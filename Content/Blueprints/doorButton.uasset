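; An interactable door button that plays a sequence and then removes a door barrier.
; Overlapping its box toggles a press-F prompt and enables input on the button, while Tick keeps the prompt oriented by the camera's position.
; F works once, disabling player character input and playing MySequence.
; When playback finishes, a bound event restores input and destroys the first DoorBarrier found and the button itself.
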(event `Key|F`
  (params (Key :type "Key Structure"))
  (bind _sequenceplayer (`LevelSequenceActor.SequencePlayer` (`self.mySequence`)))
  (:`Pressed`
    (`/Engine/EditorBlueprintResources/StandardMacros.DoOnce` false
      (:`Completed`
        (`self.DisableInput` (`GameplayStatics.GetPlayerCharacter` 0) (`GameplayStatics.GetPlayerController` 0))
        (`SceneComponent.ToggleVisibility` (`self.Press F to activate`) false)
        (`MovieSceneSequencePlayer.Play` _sequenceplayer)
        (add `MovieSceneSequencePlayer.OnFinished` _sequenceplayer (delegate `Re-enable`))))))

(event `Re-enable`
  (`SceneComponent.ToggleVisibility` (`self.Press F to activate`) false)
  (`self.EnableInput` (`GameplayStatics.GetPlayerCharacter` 0) (`GameplayStatics.GetPlayerController` 0))
  (bind _outactors (`GameplayStatics.GetAllActorsOfClass` "/Game/Blueprints/doorBarrier.doorBarrier_C"))
  (`self.K2_DestroyActor` (`|GetArrayItem` _outactors))
  (`self.K2_DestroyActor`))

(event `self.Box.OnComponentBeginOverlap`
  (params (OverlappedComponent :type "PrimitiveComponent Object Reference") (OtherActor :type "Actor Object Reference") (OtherComp :type "PrimitiveComponent Object Reference") (OtherBodyIndex :type Integer) (bFromSweep :type Boolean) (SweepResult :type "HitResult Structure (by ref)"))
  (`self.EnableInput` (`GameplayStatics.GetPlayerController` 0))
  (`SceneComponent.ToggleVisibility` (`self.Press F to activate`) false :!label _label))

(event `self.Box.OnComponentEndOverlap`
  (params (OverlappedComponent :type "PrimitiveComponent Object Reference") (OtherActor :type "Actor Object Reference") (OtherComp :type "PrimitiveComponent Object Reference") (OtherBodyIndex :type Integer))
  (`self.DisableInput` (`GameplayStatics.GetPlayerController` 0))
  (goto _label))

(event `self.ReceiveTick`
  (params (DeltaSeconds :type "Float (single-precision)"))
  (bind _press_f_to_activate (`self.Press F to activate`))
  (`SceneComponent.K2_SetRelativeRotation` _press_f_to_activate (`KismetMathLibrary.ComposeRotators` (`KismetMathLibrary.MakeRotFromX` (- (`SceneComponent.K2_GetComponentLocation` _press_f_to_activate) (`self.K2_GetActorLocation` (`GameplayStatics.GetPlayerCameraManager` 0)))) (struct :`Yaw` 10.0)) false false))

(fn `UserConstructionScript`)